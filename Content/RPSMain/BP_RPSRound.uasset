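; BP_RPSRound keeps the history of rounds for what appears to be a rock-paper-scissors game.
; AppendRound packs the player choice, opponent choice and status into a BPSRound struct and adds it to the Rounds array.
; Getter functions return the last round, the round at a given index, or all rounds matching a status filter.
; The lookups by last entry and by index read the array without bounds or empty checks.
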(event `self.AppendRound`
  (params (PlayerChoice :type "EType Enum" :default "None") (OppChoice :type "EType Enum" :default "None") (Status :type "EStatus Enum" :default "Pending"))
  (`KismetArrayLibrary.Array_Add` (`self.Rounds`) (make `/Game/RPSMain/BPS_Round` PlayerChoice OppChoice Status)))

(fn `GetLastRound`
  (returns (LastRound :type "/Game/RPSMain/BPS_Round Structure"))
  (bind _rounds (`self.Rounds`))
  (return (`|GetArrayItem` _rounds (`KismetArrayLibrary.Array_LastIndex` _rounds))))

(fn `GetRoundAtIndex`
  (params (Index :type Integer))
  (returns (Round :type "/Game/RPSMain/BPS_Round Structure"))
  (return (`|GetArrayItem` (`self.Rounds`) Index)))

(fn `GetRoundsByStatus`
  (params (StatusFilter :type "EStatus Enum" :default "Pending"))
  (returns (Rounds :type "Array of /Game/RPSMain/BPS_Round Structure"))
  (locals (RoundsWithFilter :type "Array of /Game/RPSMain/BPS_Round Structure"))
  (for _array_element (`self.Rounds`)
    (if (`|EnumEquality` (`.RoundStatus_7_ED83EE89483EDCE10EB4C3AA57736636` (break `/Game/RPSMain/BPS_Round` _array_element)) (`local.StatusFilter`))
      (`KismetArrayLibrary.Array_Add` (`local.RoundsWithFilter`) _array_element)))
  (return (`local.RoundsWithFilter`)))