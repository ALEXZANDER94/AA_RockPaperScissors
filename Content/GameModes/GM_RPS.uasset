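; Rock-paper-scissors game mode that stages each round's Level Sequence animations and bridges C++ calls to the HUD widget.
; RoundSequencer plays the camera and both choice sequences, then after the opponent sequence's duration OppositionSequencer plays the winner's opposition sequence, or none on a draw.
; Cleanup reverses stored choice sequences and hands back to RPSRound, the GameInstance holding both choices.
; PlaySequenceByType maps side, phase and choice to a sequence.
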(event `self.RoundSequencer`
  ;[1 1 1] Function to Run the Choice Sequences for the Round
  (bind (_outactor _returnvalue) (`LevelSequencePlayer.CreateLevelSequencePlayer` "/Game/RPSMain/Sequencers/LS_RoundCamera.LS_RoundCamera" (make `MovieSceneSequencePlaybackSettings` true (struct) 1.0 0.0 false true false false true)))
  (set `self.RoundLSPlayer` _returnvalue)
  (bind _asrpsround (cast `RPSRound` (`GameplayStatics.GetGameInstance`)))
  (`|ExecutionSequence`
    (:`then_0`
      (`self.PlaySequenceByType` true false true (`RPSChoice.Type` (`PlayerPawn.GetChoiceObject` (`RPSRound.GetPlayer` _asrpsround)))))
    (:`then_1`
      (bind _sequence (`self.PlaySequenceByType` false false true (`RPSChoice.Type` (`Opp.GetChoiceObject` (`RPSRound.GetOpponent` _asrpsround)))))
      (bind (_frame _framerate) (`KismetMathLibrary.BreakQualifiedFrameTime` (`MovieSceneSequencePlayer.GetEndTime` _sequence)))
      (bind (_numerator _denominator) (`KismetMathLibrary.BreakFrameRate` _framerate))
      ;;[1 1 1] To find theduration of the player, divide the frame number by the frame rate
      (set `self.RoundSetupTime` (/ (`KismetMathLibrary.Conv_IntToDouble` (`.Value` (break `FrameNumber` _frame))) (/ (`KismetMathLibrary.Conv_IntToDouble` _numerator) (`KismetMathLibrary.Conv_IntToDouble` _denominator)))))
    (:`then_2`
      (`KismetSystemLibrary.Delay` (`self.RoundSetupTime`))
      (`self.OppositionSequencer`))))

(event `self.ReceiveBeginPlay`
  ;[1 1 1] Set UI Widget
  (bind _returnvalue (`|CreateWidget` "/Game/RPSMain/HUD/UWP_UI.UWP_UI_C"))
  (bind _output_get (set `self.HUD` _returnvalue))
  (`UserWidget.AddToViewport` _output_get 0))

(event `self.ToggleRoundResult`
  ;[1 1 1] These Events exist only to link the C++ to the User Widgets
  ; It's easier to call an event from C++ on the Game Mode than it is to get a refernce to the User Widget and call the function
  ;;[1 1 1] Event to Build another Round Result Log Entry
  (`/Game/RPSMain/HUD/UWP_UI.ToggleRoundResult` (`self.HUD`)))

(event `self.ShowGameOver`
  (params (gameStatus :type "EStatus Enum" :default "Pending"))
  (bind _returnvalue (`GameplayStatics.GetPlayerController` 0))
  (bind _hud (`self.HUD`))
  ;[1 1 1] These Events exist only to link the C++ to the User Widgets
  ; It's easier to call an event from C++ on the Game Mode than it is to get a refernce to the User Widget and call the function
  ;;[1 1 1] Event to Show the GameOver HUD Element
  (`/Game/RPSMain/HUD/UWP_UI.ShowGameOver` _hud gameStatus)
  (`WidgetBlueprintLibrary.SetInputMode_UIOnlyEx` _returnvalue _hud)
  (set `PlayerController.bShowMouseCursor` true _returnvalue))

(event `OppositionSequencer`
  ;[1 1 1] Event to Run the Level Sequence that corresponds to an Opposition
  (bind _asrpsround (cast `RPSRound` (`GameplayStatics.GetGameInstance`)))
  (bind _returnvalue (`PlayerPawn.GetChoiceObject` (`RPSRound.GetPlayer` _asrpsround)))
  (if (== (`RPSChoice.Type` (`Opp.GetChoiceObject` (`RPSRound.GetOpponent` _asrpsround))) (`RPSChoice.AdvantageOver` _returnvalue))
    ;;[1 1 1] Run Opposition Sequence for Player Object
    (bind _sequence (`self.PlaySequenceByType` true true false (`RPSChoice.Type` _returnvalue)))
    (add `MovieSceneSequencePlayer.OnStop` _sequence (delegate `self.CleanupSequencer`))
    (else
      (bind _returnvalue_2 (`Opp.GetChoiceObject` (`RPSRound.GetOpponent` _asrpsround)))
      (if (== (`RPSChoice.Type` (`PlayerPawn.GetChoiceObject` (`RPSRound.GetPlayer` _asrpsround))) (`RPSChoice.AdvantageOver` _returnvalue_2))
        ;;[1 1 1] Run Opposition Sequencefor Opponent Object
        (bind _sequence_2 (`self.PlaySequenceByType` false true false (`RPSChoice.Type` _returnvalue_2)))
        (add `MovieSceneSequencePlayer.OnStop` _sequence_2 (delegate `self.CleanupSequencer`))
        (else
          ;;[1 1 1] If False, Do Cleanup Round Anim and Resolve
          (`MovieSceneSequencePlayer.PlayReverse` (`self.RoundLSPlayer`))
          (`self.CleanupSequencer`))))))

(event `self.MoveLogUp`
  ;[1 1 1] These Events exist only to link the C++ to the User Widgets
  ; It's easier to call an event from C++ on the Game Mode than it is to get a refernce to the User Widget and call the function
  (`/Game/RPSMain/HUD/UWP_UI.MoveLog` (`self.HUD`) -1.0))

(event `self.MoveLogDown`
  ;[1 1 1] These Events exist only to link the C++ to the User Widgets
  ; It's easier to call an event from C++ on the Game Mode than it is to get a refernce to the User Widget and call the function
  (`/Game/RPSMain/HUD/UWP_UI.MoveLog` (`self.HUD`) 1.0))

(event `self.CleanupSequencer`
  (bind _sequences (`self.Sequences`))
  ;[1 1 1] Cleanup Sequences - Back to C++ Functions
  ; Reverse the Setup Sequences, Clear the Sequences Array
  (for _array_element _sequences
    (`MovieSceneSequencePlayer.PlayReverse` _array_element))
  (`KismetArrayLibrary.Array_Clear` _sequences)
  (bind _asrpsround (cast `RPSRound` (`GameplayStatics.GetGameInstance`)))
  (`RPSRound.CleanupRoundAnim` _asrpsround))

(fn `PlaySequenceByType`
  (params (bPlayer :type Boolean) (Opposition :type Boolean) (Store :type Boolean) (Type :type "EType Enum" :default "Rock"))
  (returns (Sequence :type "LevelSequencePlayer Object Reference"))
  (locals (AnimSequence :type "LevelSequencePlayer Object Reference"))
  (bind _moviescenesequenceplaybacksettings (make `MovieSceneSequencePlaybackSettings` false))
  (bind _moviescenesequenceplaybacksettings_2 (make `MovieSceneSequencePlaybackSettings` false))
  (bind _moviescenesequenceplaybacksettings_3 (make `MovieSceneSequencePlaybackSettings` false))
  (bind _moviescenesequenceplaybacksettings_4 (make `MovieSceneSequencePlaybackSettings` false))
  (bind _animsequence (`local.AnimSequence`))
  (if bPlayer
    (if (`local.Opposition`)
      (switch `EType` (`local.Type`)
        (:`Rock`
          (bind (_outactor _returnvalue) (`LevelSequencePlayer.CreateLevelSequencePlayer` "/Game/RPSMain/Sequencers/Player/Opposition/LS_Player_Opposition_Rock.LS_Player_Opposition_Rock" _moviescenesequenceplaybacksettings_3))
          (set `local.AnimSequence` _returnvalue))
        (:`Paper`
          (bind (_outactor_2 _returnvalue_2) (`LevelSequencePlayer.CreateLevelSequencePlayer` "/Game/RPSMain/Sequencers/Player/Opposition/LS_Player_Opposition_Paper.LS_Player_Opposition_Paper" _moviescenesequenceplaybacksettings_3))
          (set `local.AnimSequence` _returnvalue_2))
        (:`Scissors`
          (bind (_outactor_3 _returnvalue_3) (`LevelSequencePlayer.CreateLevelSequencePlayer` "/Game/RPSMain/Sequencers/Player/Opposition/LS_Player_Opposition_Scissors.LS_Player_Opposition_Scissors" _moviescenesequenceplaybacksettings_3))
          (set `local.AnimSequence` _returnvalue_3)))
      (else
        (switch `EType` (`local.Type`)
          (:`Rock`
            (bind (_outactor_4 _returnvalue_4) (`LevelSequencePlayer.CreateLevelSequencePlayer` "/Game/RPSMain/Sequencers/Player/LS_PlayerRock.LS_PlayerRock" _moviescenesequenceplaybacksettings_4))
            (set `local.AnimSequence` _returnvalue_4))
          (:`Paper`
            (bind (_outactor_5 _returnvalue_5) (`LevelSequencePlayer.CreateLevelSequencePlayer` "/Game/RPSMain/Sequencers/Player/LS_PlayerPaper.LS_PlayerPaper" _moviescenesequenceplaybacksettings_4))
            (set `local.AnimSequence` _returnvalue_5))
          (:`Scissors`
            (bind (_outactor_6 _returnvalue_6) (`LevelSequencePlayer.CreateLevelSequencePlayer` "/Game/RPSMain/Sequencers/Player/LS_PlayerScissors.LS_PlayerScissors" _moviescenesequenceplaybacksettings_4))
            (set `local.AnimSequence` _returnvalue_6)))))
    (elif (`local.Opposition`)
      (switch `EType` (`local.Type`)
        (:`Rock`
          (bind (_outactor_7 _returnvalue_7) (`LevelSequencePlayer.CreateLevelSequencePlayer` "/Game/RPSMain/Sequencers/Opponent/Opposition/LS_OpponentOpposition_Rock.LS_OpponentOpposition_Rock" _moviescenesequenceplaybacksettings_2))
          (set `local.AnimSequence` _returnvalue_7))
        (:`Paper`
          (bind (_outactor_8 _returnvalue_8) (`LevelSequencePlayer.CreateLevelSequencePlayer` "/Game/RPSMain/Sequencers/Opponent/Opposition/LS_OpponentOpposition_Paper.LS_OpponentOpposition_Paper" _moviescenesequenceplaybacksettings_2))
          (set `local.AnimSequence` _returnvalue_8))
        (:`Scissors`
          (bind (_outactor_9 _returnvalue_9) (`LevelSequencePlayer.CreateLevelSequencePlayer` "/Game/RPSMain/Sequencers/Opponent/Opposition/LS_OpponentOpposition_Scissors.LS_OpponentOpposition_Scissors" _moviescenesequenceplaybacksettings_2))
          (set `local.AnimSequence` _returnvalue_9)))
      (else
        (switch `EType` (`local.Type`)
          (:`Rock`
            (bind (_outactor_10 _returnvalue_10) (`LevelSequencePlayer.CreateLevelSequencePlayer` "/Game/RPSMain/Sequencers/Opponent/LS_OpponentRock.LS_OpponentRock" _moviescenesequenceplaybacksettings))
            (set `local.AnimSequence` _returnvalue_10))
          (:`Paper`
            (bind (_outactor_11 _returnvalue_11) (`LevelSequencePlayer.CreateLevelSequencePlayer` "/Game/RPSMain/Sequencers/Opponent/LS_OpponentPaper.LS_OpponentPaper" _moviescenesequenceplaybacksettings))
            (set `local.AnimSequence` _returnvalue_11))
          (:`Scissors`
            (bind (_outactor_12 _returnvalue_12) (`LevelSequencePlayer.CreateLevelSequencePlayer` "/Game/RPSMain/Sequencers/Opponent/LS_OpponentScissors.LS_OpponentScissors" _moviescenesequenceplaybacksettings))
            (set `local.AnimSequence` _returnvalue_12))))))
  (if (`local.Store`)
    (`KismetArrayLibrary.Array_AddUnique` (`self.Sequences`) _animsequence))
  (`MovieSceneSequencePlayer.Play` _animsequence)
  (return _animsequence))

(fn `UserConstructionScript`)